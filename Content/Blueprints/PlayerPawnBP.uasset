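; Player pawn for a two-player networked versus game that moves vertically within screen bounds and fires an orbiting object as a projectile.
; A timeline spins the orbiter in a server-randomized direction, and shooting launches ProjectileBP along the spline tangent, hiding the orbiter until reload.
; Authority-gated damage updates health UI and, at zero, awards the opponent a round through the GameState.
; Timed power-ups double damage, projectile speed, movement speed or fire rate, then revert.
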(event `ParticleSystemActivity`
  (params (isActive :type Boolean))
  ;[1 1 1] Orbit Particle System
  (`ActorComponent.SetActive` (`self.RotationTrailParticleSystem`) isActive false))

(event `ResetPlayer`
  ;[1 1 1] Reset Player to Initial Position and State
  (`SceneComponent.K2_SetWorldLocation` (`self.DefaultSceneRoot`) (`self.OriginalLocation`) false false)
  (`self.Orbit`)
  (bind _asgravity_impact_game_state_base (cast `/Game/Blueprints/GravityImpactGameStateBase` (`GameplayStatics.GetGameState`)))
  (set `self.CurrentHealth` (`/Game/Blueprints/GravityImpactGameStateBase.PlayerMaxHealth` _asgravity_impact_game_state_base))
  (`self.UpdateHealthUI`))

(event `UpdateWinsAndRounds`
  ;[1 1 1] Update Wind and Rounds UI
  (bind _asgravity_impact_game_state_base (cast `/Game/Blueprints/GravityImpactGameStateBase` (`GameplayStatics.GetGameState`)))
  (if (`self.isServerPlayer`)
    (set `/Game/Blueprints/GravityImpactGameStateBase.Player2Wins` (+ (`/Game/Blueprints/GravityImpactGameStateBase.Player2Wins` _asgravity_impact_game_state_base) 1) _asgravity_impact_game_state_base)
    (else
      (set `/Game/Blueprints/GravityImpactGameStateBase.Player1Wins` (+ (`/Game/Blueprints/GravityImpactGameStateBase.Player1Wins` _asgravity_impact_game_state_base) 1) _asgravity_impact_game_state_base)))
  (set `/Game/Blueprints/GravityImpactGameStateBase.CurrentRound` (+ (`/Game/Blueprints/GravityImpactGameStateBase.CurrentRound` _asgravity_impact_game_state_base) 1) _asgravity_impact_game_state_base)
  (`/Game/Blueprints/GravityImpactGameStateBase.CheckForWinners` _asgravity_impact_game_state_base)
  (`/Game/Blueprints/GravityImpactGameStateBase.ResetPlayers` _asgravity_impact_game_state_base))

(event `UpdateHealthUI`
  ;[1 1 1] Update Health UI
  (bind _asgravity_impact_game_state_base (cast `/Game/Blueprints/GravityImpactGameStateBase` (`GameplayStatics.GetGameState`)))
  (`/Game/Blueprints/MainUIWB.SetPlayerHealth` (`/Game/Blueprints/GravityImpactGameStateBase.UserInformationWidget` _asgravity_impact_game_state_base) (`self.CurrentHealth`) (`self.isServerPlayer`)))

(event `self.ReceiveBeginPlay`
  ;[1 1 1] Initialization
  (`KismetSystemLibrary.Delay` 0.002)
  (set `self.OriginalLocation` (`SceneComponent.K2_GetComponentLocation` (`self.DefaultSceneRoot`)))
  (`self.ResetPlayer`))

(event `Orbit`
  ;[1 1 1] Start Orbiting in random direction and starting at a random point
  (`/Engine/EditorBlueprintResources/ActorMacros.Switch Has Authority`
    (:`Authority`
      (bind (_isreverse _startingangle) (`self.GenerateRandomOrbit`))
      (if _isreverse
        (`|ExecutionSequence`
          (:`then_0`
            (bind (_direction _pitchvalue) (`Timeline|Orbit Timeline` :`NewTime` (* (/ _startingangle 360.0) (`self.OrbitTime`)) :!via `Reverse` :!label _label)
              (:`Update`
                (`SceneComponent.K2_SetRelativeRotation` (`self.RotatingSphere`) (`KismetMathLibrary.MakeRotator` 0.0 _pitchvalue) false false)
                (set `self.ShootingDirection` (select `ETimelineDirection` _direction :`Forward` 1.0 :`Backward` -1.0 :!type "Float (single-precision)")))))
          (:`then_1`
            (goto _label :!via `SetNewTime`)))
        (else
          (`|ExecutionSequence`
            (:`then_0`
              (goto _label))
            (:`then_1`
              (goto _label :!via `SetNewTime`))))))))

(event `TangentShoot`
  ;[1 1 1] Shoot
  (if (`self.CanShoot`)
    (set `self.CanShoot` false)
    (bind _returnvalue (`|SpawnActorFromClass` "/Game/Blueprints/ProjectileBP.ProjectileBP_C" (`SceneComponent.K2_GetComponentToWorld` (`self.OrbitObject`)) "Undefined" "OverrideRootScale" null null))
    (`self.PlaySound` "/Game/Sounds/cycle-fired.cycle-fired")
    (set `/Game/Blueprints/ProjectileBP.SpawnedByPlayer` self _returnvalue)
    (set `/Game/Blueprints/ProjectileBP.Damage` (`self.Damage`) _returnvalue)
    (`SceneComponent.SetVisibility` (`self.OrbitObject`) false false)
    (`self.ParticleSystemActivity` false)
    (`/Game/Blueprints/ProjectileBP.Shoot` _returnvalue (* (`SplineComponent.GetDirectionAtSplinePoint` (`self.Tangent`) 1 "World") (`self.ShootingDirection`)) (`self.ProjectileSpeedMultiplier`))
    (set `self.CurrentPowerUp` "NewEnumerator4")
    (`KismetSystemLibrary.Delay` (`self.ReloadTime`))
    (set `self.CanShoot` true)
    (`SceneComponent.SetVisibility` (`self.OrbitObject`) true false)
    (`self.ParticleSystemActivity` true)
    (`self.Orbit`)))

(event `MoveZ`
  (params (MoveDirectrion :type "Float (double-precision)"))
  (bind _dontmoveoffset (`self.DontMoveOffset`))
  (bind (_x _y) (`KismetMathLibrary.BreakVector2D` (`WidgetLayoutLibrary.GetViewportSize`)))
  (bind _returnvalue (/ _y 10.0))
  ;[1 1 1] Move Up and Down
  (if (`self.canMove`)
    (bind _asgravity_impact_controller (cast `/Game/Blueprints/GravityImpactController` (`GameplayStatics.GetPlayerController` 0)))
    (bind (_x_2 _y_2) (`KismetMathLibrary.BreakVector2D` (`GameplayStatics.ProjectWorldToScreen` _asgravity_impact_controller (`self.K2_GetActorLocation`))))
    (if (not (or (and (> _y_2 (- (- _y _returnvalue) _dontmoveoffset)) (== MoveDirectrion -1.0)) (and (< _y_2 (+ _returnvalue _dontmoveoffset)) (== MoveDirectrion 1.0))))
      (set `MovementComponent.Velocity` (`KismetMathLibrary.MakeVector` 0.0 0.0 (* MoveDirectrion (`self.Speed`))) (`self.FloatingPawnMovement`)))))

(event `PlaySound`
  (params (SoundToPlay :type "SoundBase Object Reference"))
  ;[1 1 1] PlaySound On All Clients
  (bind _asgravity_impact_game_instance (cast `/Game/MainMenu/GravityImpactGameInstance` (`GameplayStatics.GetGameInstance`)))
  (`GameplayStatics.PlaySound2D` SoundToPlay (`/Game/MainMenu/GravityImpactGameInstance.SoundVolume` _asgravity_impact_game_instance) 1.0 0.0 null null))

(event `PowerUpHandler`
  (params (PowerUp :type "/Game/PowerUps/PowerUpTypes Enum" :default "NewEnumerator0"))
  ;[1 1 1] Power UP handler
  (switch `/Game/PowerUps/PowerUpTypes` PowerUp
    (:`NewEnumerator0`
      (`self.HandleDoubleDamgePowerUp`)
      (`KismetSystemLibrary.Delay` (`self.DoubleDamagePowerUpTime`)))
    (:`NewEnumerator1`
      (`self.HandleDoubleProjectileSpeedPowerUp`)
      (`KismetSystemLibrary.Delay` (`self.DoubleProjectileSpeedUpTime`)))
    (:`NewEnumerator2`
      (`self.HandleDoubleMovementSpeedPowerup`)
      (`KismetSystemLibrary.Delay` (`self.MovementSpeedPowerUpTime`)))
    (:`NewEnumerator3`
      (`self.HandleDoubleFireRatePowerUp`)
      (`KismetSystemLibrary.Delay` (`self.FireRatePowerUpTime`))))
  (`GameplayStatics.PlaySound2D` "/Game/Sounds/lose-powerup.lose-powerup" 1.0 1.0 0.0 null null))

(event `HandleDoubleMovementSpeedPowerup`
  ;[1 1 1] Movement Speed Power Up Handler
  (set `self.Speed` (* (`self.Speed`) 2.0))
  (`KismetSystemLibrary.Delay` (`self.MovementSpeedPowerUpTime`))
  (set `self.Speed` (/ (`self.Speed`) 2.0)))

(event `HandleDoubleFireRatePowerUp`
  ;[1 1 1] Fire Rate Power Up Handler
  (set `self.ReloadTime` (/ (`self.ReloadTime`) 2.0))
  (`KismetSystemLibrary.Delay` (`self.FireRatePowerUpTime`))
  (set `self.ReloadTime` (* (`self.ReloadTime`) 2.0)))

(event `HandleDoubleDamgePowerUp`
  ;[1 1 1] Double Damage Power Up Handler
  (set `self.Damage` (* (`self.Damage`) 2))
  (`KismetSystemLibrary.Delay` (`self.DoubleDamagePowerUpTime`))
  (set `self.Damage` (/ (`self.Damage`) 2)))

(event `HandleDoubleProjectileSpeedPowerUp`
  ;[1 1 1] Double Projectile Speed Power Up Handler
  (set `self.ProjectileSpeedMultiplier` (* (`self.ProjectileSpeedMultiplier`) 2.0))
  (`KismetSystemLibrary.Delay` (`self.DoubleProjectileSpeedUpTime`))
  (set `self.ProjectileSpeedMultiplier` (/ (`self.ProjectileSpeedMultiplier`) 2.0)))

(event `OldMoveZ`
  (params (MoveDirectrion :type "Float (double-precision)"))
  ;[1 1 1] Old Move Z
)

(fn `GenerateRandomOrbit`
  (returns (IsReverse :type Boolean) (StartingAngle :type "Float (double-precision)"))
  (return (`KismetMathLibrary.RandomBool`) (`KismetMathLibrary.RandomFloatInRange` 0.0 360.0)))

(fn `RespawnOrbitingObject`)

(fn `SubstractHealth`
  (params (Damage :type Integer))
  (`/Engine/EditorBlueprintResources/ActorMacros.Switch Has Authority`
    (:`Authority`
      (bind _output_get (set `self.CurrentHealth` (`KismetMathLibrary.Max` (- (`self.CurrentHealth`) Damage))))
      (`self.UpdateHealthUI`)
      (if (== _output_get 0)
        (`self.UpdateWinsAndRounds`)))))

(fn `UserConstructionScript`)