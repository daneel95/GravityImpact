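; Game state for a two-player networked match of Gravity Impact, handling pawn assignment, player resets and match wins.
; On BeginPlay it shows the main UI, then gives the local controller the first pawn on authority or the second on remote, flagging which is the server player.
; ResetPlayers resets every player pawn.
; CheckForWinners detects a round-majority win, displays the winner, pauses and shows the cursor.
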(event `self.ReceiveBeginPlay`
  (bind _returnvalue (`|CreateWidget` "/Game/Blueprints/MainUIWB.MainUIWB_C"))
  (bind _output_get (set `self.UserInformationWidget` _returnvalue))
  (`UserWidget.AddToViewport` _output_get 0)
  (`/Engine/EditorBlueprintResources/ActorMacros.Switch Has Authority`
    (:`Authority`
      (bind _outactors (`GameplayStatics.GetAllActorsOfClass` "/Game/Blueprints/PlayerPawnBP.PlayerPawnBP_C"))
      (bind _asgravity_impact_controller (cast `/Game/Blueprints/GravityImpactController` (`GameplayStatics.GetPlayerController` 0)))
      (bind _output_get_2 (set `/Game/Blueprints/GravityImpactController.MyPlayer` (`|GetArrayItem` _outactors) _asgravity_impact_controller))
      (set `/Game/Blueprints/PlayerPawnBP.isServerPlayer` true _output_get_2))
    (:`Remote`
      (bind _outactors_2 (`GameplayStatics.GetAllActorsOfClass` "/Game/Blueprints/PlayerPawnBP.PlayerPawnBP_C"))
      (bind _asgravity_impact_controller_2 (cast `/Game/Blueprints/GravityImpactController` (`GameplayStatics.GetPlayerController` 0)))
      (bind _output_get_3 (set `/Game/Blueprints/GravityImpactController.MyPlayer` (`|GetArrayItem` _outactors_2 1) _asgravity_impact_controller_2))
      (set `/Game/Blueprints/PlayerPawnBP.isServerPlayer` false _output_get_3))))

(fn `CheckForWinners`
  (bind _userinformationwidget (`self.UserInformationWidget`))
  (if (>= (`self.Player1Wins`) (+ (/ (`self.NumberOfRounds`) 2) 1))
    (`KismetSystemLibrary.PrintString` "Player 1 Won the Game" true true (struct :`G` 0.66 :`B` 1.0 :`A` 1.0) 3.0)
    (`/Game/Blueprints/MainUIWB.SetWinnerText` _userinformationwidget "Player 1")
    (`GameplayStatics.SetGamePaused` true :!label _label)
    (bind _asgravity_impact_controller (cast `/Game/Blueprints/GravityImpactController` (`GameplayStatics.GetPlayerController` 0)))
    (set `PlayerController.bShowMouseCursor` true _asgravity_impact_controller)
    (elif (>= (`self.Player2Wins`) (+ (/ (`self.NumberOfRounds`) 2) 1))
      (`KismetSystemLibrary.PrintString` "Player 2 Won the Game" true true (struct :`G` 0.66 :`B` 1.0 :`A` 1.0) 3.0)
      (`/Game/Blueprints/MainUIWB.SetWinnerText` _userinformationwidget "Player 2")
      (goto _label))))

(fn `ResetPlayers`
  (bind _outactors (`GameplayStatics.GetAllActorsOfClass` "/Game/Blueprints/PlayerPawnBP.PlayerPawnBP_C"))
  (for _array_element _outactors
    (`/Game/Blueprints/PlayerPawnBP.ResetPlayer` _array_element)))

(fn `UserConstructionScript`)