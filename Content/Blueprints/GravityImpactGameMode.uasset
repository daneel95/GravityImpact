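; GravityImpactGameMode is a game mode that offers a GetPlayerPawn function for retrieving the player's pawn.
; GetPlayerPawn casts player controller 0 to GravityImpactController and returns its MyPlayer, with identical logic on both authority and remote branches.
; BeginPlay is empty.
; A disconnected, never-run block would set MyPlayer to the first PlayerPawnBP actor on authority and the second on remote.
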(event `self.ReceiveBeginPlay`)

(fn `GetPlayerPawn`
  (returns (PlayerPawn :type "/Game/Blueprints/PlayerPawnBP Object Reference"))
  (`/Engine/EditorBlueprintResources/ActorMacros.Switch Has Authority`
    (:`Authority`
      (bind _asgravity_impact_controller (cast `/Game/Blueprints/GravityImpactController` (`GameplayStatics.GetPlayerController` 0)))
      (return (`/Game/Blueprints/GravityImpactController.MyPlayer` _asgravity_impact_controller)))
    (:`Remote`
      (bind _asgravity_impact_controller_2 (cast `/Game/Blueprints/GravityImpactController` (`GameplayStatics.GetPlayerController` 0)))
      (return (`/Game/Blueprints/GravityImpactController.MyPlayer` _asgravity_impact_controller_2)))))

(fn `UserConstructionScript`)