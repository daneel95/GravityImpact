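; Level background music player for Gravity Impact that cycles endlessly through a list of tracks.
; On BeginPlay it sets the Audio component's volume from the game instance's SoundVolume and plays the track at the current index.
; Each finished track triggers the next through the audio-finished delegate, wrapping around at the list's end.
; A SetSoundVolume event allows the volume to be changed at runtime.
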(event `SetSoundVolume`
  (params (Volume :type "Float (double-precision)"))
  (`AudioComponent.SetVolumeMultiplier` (`self.Audio`) Volume))

(event `self.ReceiveBeginPlay`
  (bind _audio (`self.Audio`))
  (bind _audiolist (`self.AudioList`))
  (bind _soundindex (`self.SoundIndex`))
  (bind _asgravity_impact_game_instance (cast `/Game/MainMenu/GravityImpactGameInstance` (`GameplayStatics.GetGameInstance`)))
  (`AudioComponent.SetVolumeMultiplier` (`self.Audio`) (`/Game/MainMenu/GravityImpactGameInstance.SoundVolume` _asgravity_impact_game_instance))
  (`AudioComponent.SetSound` _audio (`|GetArrayItem` _audiolist _soundindex) :!label _label)
  (set `self.SoundIndex` (mod (+ _soundindex 1) (`KismetArrayLibrary.Array_Length` _audiolist)))
  (add `AudioComponent.OnAudioFinished` _audio (delegate `OnAudioFinished_Event_0`))
  (`AudioComponent.Play` _audio 0.0))

(event `OnAudioFinished_Event_0`
  (goto _label))

(fn `UserConstructionScript`)