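; Projectile actor that damages player pawns it hits, ignoring the player who spawned it.
; Shoot sets the projectile movement velocity along a given direction at a set speed.
; On overlap with another player, it subtracts health, plays a hit sound, spawns a small explosion and destroys itself after a brief delay.
; Overlapping an invisible wall destroys it immediately; other actors are ignored.
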(event `self.ReceiveActorBeginOverlap`
  (params (OtherActor :type "Actor Object Reference"))
  (bind _asplayer_pawn_bp (cast `/Game/Blueprints/PlayerPawnBP` OtherActor)
    (:`then`
      (if (!= _asplayer_pawn_bp (`self.SpawnedByPlayer`))
        (`/Game/Blueprints/PlayerPawnBP.SubstractHealth` _asplayer_pawn_bp (`self.Damage`))
        (`GameplayStatics.PlaySound2D` "/Game/Sounds/enemy-hit.enemy-hit" 1.0 1.0 0.0 null null)
        (`GameplayStatics.SpawnEmitterAtLocation` "/Game/Particles/ProjectileExplosion.ProjectileExplosion" (`SceneComponent.K2_GetComponentLocation` (`self.DefaultSceneRoot`)) (struct) (0.3 0.3 0.3))
        (`KismetSystemLibrary.Delay` 0.05)
        (`self.K2_DestroyActor`)))
    (:`CastFailed`
      (cast `/Game/Blueprints/InvisibleWall` OtherActor)
      (`self.K2_DestroyActor`))))

(fn `Shoot`
  (params (ForwardVector :type "Vector Structure"))
  (set `MovementComponent.Velocity` (* (`KismetMathLibrary.Normal` ForwardVector) (`self.Speed`)) (`self.ProjectileMovement`)))

(fn `UserConstructionScript`)